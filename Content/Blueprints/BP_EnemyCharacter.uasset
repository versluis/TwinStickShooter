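; BP_EnemyCharacter is a twin-stick shooter enemy that damages the hero on contact and awards score when killed.
; Overlapping the hero starts a looping timer that applies damage at its attack rate until the overlap ends.
; On death it disables Pawn and WorldDynamic collision, reports score to the game mode, detaches its controller, then after a delay spawns an explosion and destroys itself.
; The construction script tints the body through a dynamic material.
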(event `self.AffectHealth`
  (params (Delta :type "Float (single-precision)"))
  (bind _capsulecomponent (`self.CapsuleComponent`))
  (`self.CalculateHealth` Delta)
  (if (`self.bIsDead`)
    (`PrimitiveComponent.SetCollisionResponseToChannel` _capsulecomponent "ECC_WorldDynamic" "ECR_Ignore")
    (`PrimitiveComponent.SetCollisionResponseToChannel` _capsulecomponent "ECC_Pawn" "ECR_Ignore")
    (bind _asbp_twin_stick_mode (cast `/Game/Blueprints/BP_TwinStickMode` (`GameplayStatics.GetGameMode`)))
    (`/Game/Blueprints/BP_TwinStickMode.IncrementScore` _asbp_twin_stick_mode (`self.Score`))
    (`self.DetachFromControllerPendingDestroy`)
    (`KismetSystemLibrary.Delay` (`self.TimeToDestroyDeadEnemy`))
    (`|SpawnActorFromClass` "/Game/Blueprints/BP_EnemyExplosion.BP_EnemyExplosion_C" (`self.GetTransform`) "Undefined" "OverrideRootScale" null null)
    (`self.K2_DestroyActor`)))

(event `self.ReceiveActorBeginOverlap`
  (params (OtherActor :type "Actor Object Reference"))
  (bind _asbp_hero_character (cast `/Game/Blueprints/BP_HeroCharacter` OtherActor))
  (set `self.Hero` _asbp_hero_character)
  (`KismetSystemLibrary.K2_SetTimer` null "DamageHero" (/ 1.0 (`self.AttacksPerSecond`)) true))

(event `self.ReceiveActorEndOverlap`
  (params (OtherActor :type "Actor Object Reference"))
  (if (== OtherActor (`self.Hero`))
    (`KismetSystemLibrary.K2_ClearTimer` null "DamageHero")))

(event `DamageHero`
  (`self.AffectHealth` (`self.Hero`) (`self.Damage`)))

(fn `UserConstructionScript`
  (bind _returnvalue (`PrimitiveComponent.CreateDynamicMaterialInstance` (`self.Mesh`) 0 null "None"))
  (bind _output_get (set `self.DynaMat` _returnvalue))
  (`MaterialInstanceDynamic.SetVectorParameterValue` _output_get "BodyColor" (`self.EnemyBodyColor`)))